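; BP_Teleport3 is a teleporter actor that sends the player character to the level's BP_ArtMap03 actor.
; BeginPlay caches that actor, and clicking the Button component teleports the player to 50 units above its root location.
; A Box overlap shows the button when the player enters, and any end overlap hides it.
; The construction script positions an Arrow from TeleportLocation, which the teleport itself does not use.
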(event `self.ReceiveBeginPlay`
  (`|ExecutionSequence`
    (:`then_2`
      (bind _returnvalue (`GameplayStatics.GetActorOfClass` "/Game/ArtProject/LHM/BluePrints/BP_ArtMap03.BP_ArtMap03_C"))
      (set `self.Level3` _returnvalue))))

(event `self.Button.OnClicked`
  (params (TouchedComponent :type "PrimitiveComponent Object Reference") (ButtonPressed :type "Key Structure"))
  (bind (_returnvalue_x _returnvalue_y _returnvalue_z) (`KismetMathLibrary.BreakVector` (`SceneComponent.K2_GetComponentLocation` (`Actor.RootComponent` (`self.Level3`)))))
  ;[1 1 1] Clicked Teleport
  (`self.K2_TeleportTo` :`self` (`GameplayStatics.GetPlayerCharacter` 0) :`DestLocation` (`KismetMathLibrary.MakeVector` _returnvalue_x _returnvalue_y (+ _returnvalue_z 50.0))))

(event `self.Box.OnComponentBeginOverlap`
  (params (OverlappedComponent :type "PrimitiveComponent Object Reference") (OtherActor :type "Actor Object Reference") (OtherComp :type "PrimitiveComponent Object Reference") (OtherBodyIndex :type Integer) (bFromSweep :type Boolean) (SweepResult :type "HitResult Structure (by ref)"))
  ;[1 1 1] Set Visibility
  (if (== OtherActor (`GameplayStatics.GetPlayerCharacter` 0))
    (`SceneComponent.SetVisibility` (`self.Button`) true false)))

(event `self.Box.OnComponentEndOverlap`
  (params (OverlappedComponent :type "PrimitiveComponent Object Reference") (OtherActor :type "Actor Object Reference") (OtherComp :type "PrimitiveComponent Object Reference") (OtherBodyIndex :type Integer))
  ;[1 1 1] Set Visibility
  (`SceneComponent.SetVisibility` (`self.Button`) false false))

(fn `UserConstructionScript`
  (`SceneComponent.K2_SetRelativeTransform` (`self.Arrow`) (`self.Teleport Location`) false false))