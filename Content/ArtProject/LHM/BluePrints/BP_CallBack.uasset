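; BP_CallBack is an actor that receives exported Niagara particle data and uses it to trigger destruction of a BP_Text actor.
; On BeginPlay it registers itself as the Niagara User.BPCallBack object and finds the BP_Text actor.
; For each particle received, it prints position tinted by velocity, then destroys the text if this actor is at least as near the world origin.
; That distance test ignores particle position, using only the two actors' locations.
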(event `self.ReceiveBeginPlay`
  (`NiagaraComponent.SetNiagaraVariableObject` (`self.Niagara`) "User.BPCallBack" self)
  (bind _returnvalue (`GameplayStatics.GetActorOfClass` "/Game/ArtProject/LHM/BluePrints/BP_Text.BP_Text_C"))
  (set `self.Text` _returnvalue))

(event `self.ReceiveParticleData`
  (params (Data :type "Array of BasicParticleData Structure (by ref)") (NiagaraSystem :type "NiagaraSystem Object Reference") (SimulationPositionOffset :type "Vector Structure (by ref)"))
  (bind _text (`self.Text`))
  (for _array_element Data
    (bind (_position _size _velocity) (break `BasicParticleData` _array_element))
    (`KismetSystemLibrary.PrintString` (`KismetStringLibrary.Conv_VectorToString` _position) true true (`KismetMathLibrary.Conv_VectorToLinearColor` _velocity))
    (if (<= (`KismetMathLibrary.Vector_Distance` (`self.K2_GetActorLocation`)) (`KismetMathLibrary.Vector_Distance` (`self.K2_GetActorLocation` _text)))
      (`/Engine/EditorBlueprintResources/StandardMacros.IsValid` _text
        (:`Is Valid`
          (`self.K2_DestroyActor` _text)
          (`KismetSystemLibrary.PrintString` "Succeded")))
      (else
        (`KismetSystemLibrary.PrintString` "Failed....")))))

(fn `UserConstructionScript`)