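; BP_ArtPlayer is an art-project player whose head and hand smoke particles knock scene components away, then hide them.
; On BeginPlay it registers itself as the Niagara export callback and blends the view to the "camera1"-tagged camera.
; ParticleData runs three height-staggered, debug-drawn sphere traces along Y from each particle position, separated by short delays.
; Hits receive randomized-X impulses, then after a delay lose physics, collision and visibility.
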(event `self.ReceiveBeginPlay`
  (`NiagaraComponent.SetNiagaraVariableObject` (`self.SmokeNiagaraOnHeadComp`) "User.BPCallBack" self)
  (`NiagaraComponent.SetNiagaraVariableObject` (`self.SmokeNiagaraOnLHandComp`) "User.BPCallBack" self)
  (`NiagaraComponent.SetNiagaraVariableObject` (`self.SmokeNiagaraOnRHandComp`) "User.BPCallBack" self)
  (bind _outactors (`GameplayStatics.GetAllActorsOfClassWithTag` "/Script/Engine.CameraActor" "camera1"))
  (for _array_element _outactors
    (`PlayerController.SetViewTargetWithBlend` (`GameplayStatics.GetPlayerController` 0) _array_element 1.0 "VTBlend_Linear" 0.0 false)))

(event `self.ReceiveParticleData`
  (params (Data :type "Array of BasicParticleData Structure (by ref)") (NiagaraSystem :type "NiagaraSystem Object Reference") (SimulationPositionOffset :type "Vector Structure (by ref)"))
  (for _array_element Data
    (bind _position (break `BasicParticleData` _array_element))
    (bind _returnvalue (+ (.y _position) 50.0))
    (bind _returnvalue_2 (- (.y _position) 100.0))
    ;[1 1 1] Comment
    (bind _outhits (`KismetSystemLibrary.SphereTraceMulti` :`Start` (`KismetMathLibrary.MakeVector` (.x _position) _returnvalue (.z _position)) :`End` (`KismetMathLibrary.MakeVector` (.x _position) _returnvalue_2 (.z _position)) :`Radius` (`self.SphereTraceRadius`) :`TraceChannel` "TraceTypeQuery3" :`DrawDebugType` "ForOneFrame"))
    (for _array_element_2 _outhits
      (bind (_bblockinghit _binitialoverlap _time _distance _location _impactpoint _normal _impactnormal _physmat _hitactor _hitcomponent) (`GameplayStatics.BreakHitResult` _array_element_2))
      (`/Engine/EditorBlueprintResources/StandardMacros.IsValid` _hitcomponent
        (:`Is Valid`
          (bind _output_get (set `self.force` (`KismetMathLibrary.MakeVector` (`KismetMathLibrary.RandomFloatInRange` (`self.Force_Min`) (`self.Force_Max`)) 0.0 (`self.Force_Z`))))
          (`PrimitiveComponent.AddImpulse` _hitcomponent _output_get "None" false)
          (`KismetSystemLibrary.Delay` 1.0)
          (`/Engine/EditorBlueprintResources/StandardMacros.IsValid` _hitcomponent
            (:`Is Valid`
              (`PrimitiveComponent.SetSimulatePhysics` _hitcomponent false)
              (`PrimitiveComponent.SetCollisionEnabled` _hitcomponent "NoCollision")
              (`SceneComponent.SetVisibility` _hitcomponent false false)
              (`KismetSystemLibrary.PrintString` (`KismetSystemLibrary.GetDisplayName` _hitcomponent)))))))
    (`KismetSystemLibrary.Delay` 0.2)
    (bind _returnvalue_3 (+ (.z _position) 50.0))
    ;[1 1 1] Comment
    (bind _outhits_2 (`KismetSystemLibrary.SphereTraceMulti` :`Start` (`KismetMathLibrary.MakeVector` (.x _position) _returnvalue _returnvalue_3) :`End` (`KismetMathLibrary.MakeVector` (.x _position) _returnvalue_2 _returnvalue_3) :`Radius` (`self.SphereTraceRadius`) :`TraceChannel` "TraceTypeQuery3" :`DrawDebugType` "ForOneFrame"))
    (for _array_element_3 _outhits_2
      (bind (_bblockinghit_2 _binitialoverlap_2 _time_2 _distance_2 _location_2 _impactpoint_2 _normal_2 _impactnormal_2 _physmat_2 _hitactor_2 _hitcomponent_2) (`GameplayStatics.BreakHitResult` _array_element_3))
      (`/Engine/EditorBlueprintResources/StandardMacros.IsValid` _hitcomponent_2
        (:`Is Valid`
          (bind _output_get_2 (set `self.force` (`KismetMathLibrary.MakeVector` (`KismetMathLibrary.RandomFloatInRange` (`self.Force_Min`) (`self.Force_Max`)) 0.0 (`self.Force_Z`))))
          (`PrimitiveComponent.AddImpulse` _hitcomponent_2 _output_get_2 "None" false)
          (`KismetSystemLibrary.Delay` 1.0)
          (`/Engine/EditorBlueprintResources/StandardMacros.IsValid` _hitcomponent_2
            (:`Is Valid`
              (`PrimitiveComponent.SetSimulatePhysics` _hitcomponent_2 false)
              (`PrimitiveComponent.SetCollisionEnabled` _hitcomponent_2 "NoCollision")
              (`SceneComponent.SetVisibility` _hitcomponent_2 false false)
              (`KismetSystemLibrary.PrintString` (`KismetSystemLibrary.GetDisplayName` _hitcomponent_2)))))))
    (`KismetSystemLibrary.Delay` 0.2)
    (bind _returnvalue_4 (+ (.z _position) 100.0))
    ;[1 1 1] Comment
    (bind _outhits_3 (`KismetSystemLibrary.SphereTraceMulti` :`Start` (`KismetMathLibrary.MakeVector` (.x _position) _returnvalue _returnvalue_4) :`End` (`KismetMathLibrary.MakeVector` (.x _position) _returnvalue_2 _returnvalue_4) :`Radius` (`self.SphereTraceRadius`) :`TraceChannel` "TraceTypeQuery3" :`DrawDebugType` "ForOneFrame"))
    (for _array_element_4 _outhits_3
      (bind (_bblockinghit_3 _binitialoverlap_3 _time_3 _distance_3 _location_3 _impactpoint_3 _normal_3 _impactnormal_3 _physmat_3 _hitactor_3 _hitcomponent_3) (`GameplayStatics.BreakHitResult` _array_element_4))
      (`/Engine/EditorBlueprintResources/StandardMacros.IsValid` _hitcomponent_3
        (:`Is Valid`
          (bind _output_get_3 (set `self.force` (`KismetMathLibrary.MakeVector` (`KismetMathLibrary.RandomFloatInRange` (`self.Force_Min`) (`self.Force_Max`)) 0.0 (`self.Force_Z`))))
          (`PrimitiveComponent.AddImpulse` _hitcomponent_3 _output_get_3 "None" false)
          (`KismetSystemLibrary.Delay` 1.0)
          (`/Engine/EditorBlueprintResources/StandardMacros.IsValid` _hitcomponent_3
            (:`Is Valid`
              (`PrimitiveComponent.SetSimulatePhysics` _hitcomponent_3 false)
              (`PrimitiveComponent.SetCollisionEnabled` _hitcomponent_3 "NoCollision")
              (`SceneComponent.SetVisibility` _hitcomponent_3 false false)
              (`KismetSystemLibrary.PrintString` (`KismetSystemLibrary.GetDisplayName` _hitcomponent_3)))))))))

(fn `UserConstructionScript`)