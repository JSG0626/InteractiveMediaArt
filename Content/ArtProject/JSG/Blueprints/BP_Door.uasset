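; BP_Door is a double door that swings open when something overlaps its trigger sphere.
; The overlap calls Exit, which sets the Eixt flag and enables actor tick, with no filter on the overlapping actor.
; Tick eases both leaves toward fixed relative rotations by lerping from their current rotation with a delta-time alpha.
; Nothing here reads the flag, disables tick or closes the door.
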(event `self.ReceiveTick`
  (params (DeltaSeconds :type "Float (single-precision)"))
  (bind _returnvalue (* DeltaSeconds 0.5))
  (bind _leftdoor (`self.LeftDoor`))
  (`SceneComponent.K2_SetRelativeRotation` _leftdoor (`KismetMathLibrary.RLerp` (`SceneComponent.RelativeRotation` _leftdoor) (struct :`Yaw` -140.0) _returnvalue) false false)
  (`SceneComponent.K2_SetRelativeRotation` (`self.RightDoor`) (`KismetMathLibrary.RLerp` (`SceneComponent.RelativeRotation` (`self.RightDoor`)) (struct :`Yaw` 300.0) _returnvalue true) false false))

(event `self.Sphere.OnComponentBeginOverlap`
  (params (OverlappedComponent :type "PrimitiveComponent Object Reference") (OtherActor :type "Actor Object Reference") (OtherComp :type "PrimitiveComponent Object Reference") (OtherBodyIndex :type Integer) (bFromSweep :type Boolean) (SweepResult :type "HitResult Structure (by ref)"))
  (`self.Exit`))

(fn `Exit`
  (set `self.bEixt` true)
  (`self.SetActorTickEnabled` true))

(fn `UserConstructionScript`)