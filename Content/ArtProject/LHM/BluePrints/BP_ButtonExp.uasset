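; BP_ButtonExp is a clickable-button Blueprint in the art project that appears to be an unfinished teleport to the BP_ArtMap01 actor.
; BeginPlay finds and caches that actor, but the click event and construction script are empty.
; Unconnected node chains sketch visibility toggling, player teleportation slightly above the map actor, and a transform snap with control-rotation and velocity reset, none of which runs.
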(event `self.ReceiveBeginPlay`
  (`|ExecutionSequence`
    (:`then_0`
      (bind _returnvalue (`GameplayStatics.GetActorOfClass` "/Game/ArtProject/LHM/BluePrints/BP_ArtMap01.BP_ArtMap01_C"))
      (set `self.Art MAp 01` _returnvalue))))

(event `self.ReceiveActorOnClicked`
  (params (ButtonPressed :type "Key Structure")))

(event `Key|LeftMouseButton`
  (params (Key :type "Key Structure")))

(fn `UserConstructionScript`)