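; Lobby player Blueprint that records voice input for an AI docent chatbot.
; On BeginPlay it creates an HTTP widget, links it to the level's BP_CJS_HttpNetActor and sets game-only input.
; AIChatbot starts audio capture and submix recording; VoiceRecord stops it, exports a WAV, then after a short delay passes the file path to the widget to send a POST.
; ActivateAIChatbot and ActivateVoiceRecord are empty.
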(event `Key|One`
  (params (Key :type "Key Structure"))
  ;[1 1 1] AI Docent Input Key
)

(event `self.ReceiveBeginPlay`
  (bind _returnvalue (`GameplayStatics.GetPlayerController` 0))
  ;[1 1 1] 웹 통신 액터 설정
  (bind _returnvalue_2 (`|CreateWidget` "/Game/ArtProject/CJS/UI/WBP_CJS_HttpNetWidget.WBP_CJS_HttpNetWidget_C"))
  (bind _output_get (set `self.HttpNetWidget` _returnvalue_2))
  (`UserWidget.AddToViewport` _output_get 0)
  (set `PlayerController.bShowMouseCursor` false _returnvalue)
  (`WidgetBlueprintLibrary.SetInputMode_GameOnly` _returnvalue)
  (bind _returnvalue_3 (`GameplayStatics.GetActorOfClass` "/Game/ArtProject/CJS/Blueprints/BP_CJS_HttpNetActor.BP_CJS_HttpNetActor_C"))
  (`CJS_HttpNetWidget.SetHttpNetActor` (`self.HttpNetWidget`) _returnvalue_3))

(event `ActivateAIChatbot`)

(event `self.AIChatbot`
  (params (buttonexp :type "CJS_AIChatbotBnt Object Reference"))
  ;[1 1 1] Voice Recording
  (`KismetSystemLibrary.PrintString` "ActivateAlchatbot")
  (`SynthComponent.Start` (`self.AudioCapture`))
  (`AudioMixerBlueprintLibrary.StartRecordingOutput` 0.0 "/Game/ArtProject/CJS/Sounds/VoiceRecord.VoiceRecord")
  (`KismetSystemLibrary.PrintString` "Recording" true true (struct :`G` 0.66 :`B` 1.0 :`A` 1.0) 3.0 "-1"))

(event `Activate Voice Record`)

(event `self.VoiceRecord`
  (params (buttonexp :type "CJS_AIChatbotBnt Object Reference"))
  (bind _httpnetwidget (`self.HttpNetWidget`))
  ;[1 1 1] Making Wav File & Saving in Path
  (`KismetSystemLibrary.PrintString` "Activate Voice Record")
  (`SynthComponent.Stop` (`self.AudioCapture`))
  (`AudioMixerBlueprintLibrary.StopRecordingOutput` "WavFile" (`self.Name`) (`self.Path`) "/Game/ArtProject/CJS/Sounds/VoiceRecord.VoiceRecord" null)
  (`KismetSystemLibrary.PrintString` "Finished Recording" true true (struct :`G` 0.66 :`B` 1.0 :`A` 1.0) 2.0 "1")
  (`KismetSystemLibrary.Delay` 1.0)
  ;[1 1 1] HttpNet 호출
  (set `CJS_HttpNetWidget.WavFilePath` (`KismetStringLibrary.Concat_StrStr` (`self.Path`) (`self.Name`) ".wav") _httpnetwidget)
  (`CJS_HttpNetWidget.OnMyClickSendPost` _httpnetwidget))

(fn `ActivateHttpNet`
  (bind _httpnetwidget (`self.HttpNetWidget`))
  ;[1 1 1] HttpNet 호출
  (set `CJS_HttpNetWidget.WavFilePath` (`KismetStringLibrary.Concat_StrStr` (`self.Path`) (`self.Name`) ".wav") _httpnetwidget)
  (`CJS_HttpNetWidget.OnMyClickSendPost` _httpnetwidget))

(fn `UserConstructionScript`)